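; Game instance Blueprint that shows the main menu and handles hosting and joining online multiplayer sessions.
; ShowMenu adds the UW_Menu widget to the viewport and enables the mouse cursor.
; HostCreatesession creates a two-connection non-LAN session, then opens ThirdPersonMap as a listen server, or the Menu level on failure.
; JoinSession joins a supplied search result and only prints whether it connected or failed.
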(event Custom|JoinSession
  (params (SearchResult :type Blueprint%20Session%20Result%20Structure%20%28by%20ref%29))
  ;[1 1 1] Присоединится к сессии
  (|JoinSession (Game|GetPlayerController 0) SearchResult
    (:OnSuccess
      (Development|PrintString "connected"))
    (:OnFailure
      (Development|PrintString "FailConnection"))))

(event Custom|HostCreate%20session
  ;[1 1 1] Стать хостом
  (|Session (Game|GetPlayerController 0) 2 false
    (:OnSuccess
      (Game|OpenLevel(byName) "ThirdPersonMap" true "listen")
      (Variables|/Script/Engine.PlayerController|SetbShowMouseCursor (Game|GetPlayerController 0) false))
    (:OnFailure
      (Game|OpenLevel(byName) "Menu"))))

(event Custom|ShowMenu
  (bind _returnvalue (Game|GetPlayerController 0))
  ;[1 1 1] Меню
  (bind _returnvalue_2 (UserInterface|CreateWidget "/Game/Menu/UW_Menu.UW_Menu_C" _returnvalue))
  (UserInterface|Viewport|AddtoViewport _returnvalue_2 0)
  (Variables|/Script/Engine.PlayerController|SetbShowMouseCursor _returnvalue true))