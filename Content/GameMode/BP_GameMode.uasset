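; Game mode for a two-player networked brick-breaker that runs spawning and win/loss flow.
; It spawns a ball and starter block at BeginPlay and possesses each new player with a Player1 pawn; the second join launches the ball and scatters random block variants.
; Tick polls actors: no balls tears down the session and opens Menu, while no blocks shows both players UI and server-travels once the second is ready.
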(event Custom|FindSpawn
  ;[1 1 1] Локация для спавная игровка
  (bind _outactors (Actor|GetAllActorsOfClass "/Game/Players/BP_PlayerStart.BP_PlayerStart_C"))
  (Utilities|IsValid (Utilities|Array|Get(acopy) _outactors (Math|Random|RandomInteger 0))
    (:Is%20Valid
      (Variables|Default|SetLocation (Transformation|GetActorLocation (Utilities|Array|Get(acopy) _outactors (Math|Random|RandomInteger 0)))))))

(event Custom|LevelStart
  ;[1 1 1] Передача управления
  (Utilities|FlowControl|Delay 3.0)
  (for _array_element (Variables|Default|GetPCs)
    (Default|InableAllInput _array_element)))

(event Custom|Player%20ready
  ;[1 1 1] Победа и условия для нее
  (Development|ExecuteConsoleCommand (Utilities|String|Append "servertravel " "ThirdPersonMap") 0))

(event EventBeginPlay
  ;[1 1 1] Для соблюдения условий
  (bind _returnvalue (Game|SpawnActorfromClass "/Game/Ball/BP_Ball.BP_Ball_C" (Math|Transform|MakeTransform "200.000000,1200.000000,50.000000" "0, 0, 0" "1.000000,1.000000,1.000000") "Undefined" 0 0))
  (Game|SpawnActorfromClass "/Game/Blocks/BP_Block.BP_Block_C" (Math|Transform|MakeTransform "400.000000,600.000000,0.000000" "0, 0, 0" "1.000000,2.000000,1.000000") "Undefined" 0 0))

(event EventPostLogin
  (params (NewPlayer :type Player%20Controller%20Object%20Reference))
  ;[1 1 1] Когда игроки логинятся
)

(event EventTick
  (params (DeltaSeconds :type Float%20%28single-precision%29))
  (bind _pcs (Variables|Default|GetPCs))
  (bind _pcs_2 (Variables|Default|GetPCs))
  (bind _output (Utilities|Array|Get(acopy) _pcs_2 1))
  (bind _outactors (Actor|GetAllActorsOfClass "/Game/Ball/BP_Ball.BP_Ball_C"))
  (if (Utilities|Array|IsEmpty _outactors)
    ;[1 1 1] Пройгрыш
    (Utilities|FlowControl|Delay 1.0)
    (|DestroySession (Utilities|Array|Get(acopy) _pcs)
      (:OnSuccess
        (Default|EndSession (Utilities|Array|Get(acopy) _pcs 1))
        (Game|OpenLevel(byName) "Menu")))
    (else
      ;[1 1 1] Победа и условия для нее
      (bind _returnvalue (Class|GameModeBase|GetNumPlayers))
      (if (not (< _returnvalue 2))
        (bind _outactors_2 (Actor|GetAllActorsOfClass "/Game/Blocks/BP_Block.BP_Block_C"))
        (bind _outactors_3 (Actor|GetAllActorsOfClass "/Game/Blocks/BP_GreenBlock.BP_GreenBlock_C"))
        (bind _outactors_4 (Actor|GetAllActorsOfClass "/Game/Blocks/BP_RedBlock.BP_RedBlock_C"))
        (if (and (and (Utilities|Array|IsEmpty _outactors_2) (Utilities|Array|IsEmpty _outactors_3)) (Utilities|Array|IsEmpty _outactors_4))
          (Default|UIDraw (Utilities|Array|Get(acopy) _pcs_2))
          (Default|UIDraw _output)
          (Utilities|IsValid _output
            (:Is%20Valid
              (if (Variables|/Game/Players/BP_PlayerController1.BP_PlayerController1_C|GetPlayerReady _output)
                (CallFunction|PlayerReady)))))))))

(event EventHandleStartingNewPlayer
  (params (NewPlayer :type Player%20Controller%20Object%20Reference))
  (bind _spawnlocation (Variables|Default|GetSpawnLocation))
  (bind _returnvalue (Math|Random|RandomFloatinRange (.y _spawnlocation) 1.7e+03))
  (bind _returnvalue_2 (Math|Random|RandomFloatinRange 1.05e+03 (.x _spawnlocation)))
  (bind _returnvalue_3 (Math|Vector|MakeVector _returnvalue_2 _returnvalue (.z _spawnlocation)))
  (bind _returnvalue_4 (Math|Transform|MakeTransform _returnvalue_3 "0, 0, 0" "1.000000,2.000000,1.000000"))
  ;[1 1 1] Когда игроки логинятся
  (bind _asbp_player_controller_1 (Utilities|Casting|CastToBP_PlayerController1 NewPlayer))
  (Utilities|Array|Add (Variables|Default|GetPCs) _asbp_player_controller_1)
  (CallFunction|SpawnPlayer _asbp_player_controller_1)
  ;[1 1 1] Рандомная генерация уровня
  (bind _returnvalue_5 (Class|GameModeBase|GetNumPlayers))
  (if (== _returnvalue_5 2)
    ;[1 1 1] Для соблюдения условий
    (Physics|AddImpulse (Variables|/Game/Ball/BP_Ball.BP_Ball_C|GetSphere (stale EventBeginPlay _returnvalue)) "1000.000000,100.000000,0.000000" "None" true)
    (for _index (range 0 9)
      (switch int (Math|Random|RandomIntegerinRange 0 2)
        (:0
          (Game|SpawnActorfromClass "/Game/Blocks/BP_Block.BP_Block_C" _returnvalue_4 "AdjustIfPossibleButAlwaysSpawn" 0 0))
        (:1
          (Game|SpawnActorfromClass "/Game/Blocks/BP_RedBlock.BP_RedBlock_C" _returnvalue_4 "AdjustIfPossibleButAlwaysSpawn" 0 0))
        (:2
          (Game|SpawnActorfromClass "/Game/Blocks/BP_GreenBlock.BP_GreenBlock_C" _returnvalue_4 "AdjustIfPossibleButAlwaysSpawn" 0 0)))
      (Utilities|FlowControl|Delay 1.0))))

(fn ConstructionScript)

(fn ReadytoStartMatch
  (return false))

(fn SpawnPlayer
  (params (PC :type BP%20Player%20Controller%201%20Object%20Reference))
  (bind _returnvalue (Pawn|GetControlledPawn PC))
  (Utilities|IsValid _returnvalue
    (:Is%20Valid
      (Actor|DestroyActor _returnvalue))
    (:Is%20Not%20Valid
      _))
  (CallFunction|FindSpawn)
  (bind _returnvalue_2 (Game|SpawnActorfromClass "/Game/Players/Player1.Player1_C" (Math|Transform|MakeTransform (Variables|Default|GetLocation) "0, 0, 0" "1.000000,3.000000,1.000000") "AdjustIfPossibleButAlwaysSpawn" 0 0))
  (Pawn|Possess PC _returnvalue_2))