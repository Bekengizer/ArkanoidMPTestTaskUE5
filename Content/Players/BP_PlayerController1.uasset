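; Player controller for a networked game that moves a Player1 pawn sideways under a level camera set as view target shortly after BeginPlay.
; Axis input applies a swept Y offset locally; remote clients also send the movement and pawn scale through OnServer for the server to apply.
; Other events enable pawn input, store ready state, destroy the session, and show the UW_YouWin widget with cursor and game paused.
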(event Custom|EndSession
  ;[1 1 1] Конец Сессии для клиента
  (|DestroySession self))

(event Custom|UIDraw
  ;[1 1 1] Отрисовка виджета на клиентах вызывается из GameMode
  (Variables|Default|SetbShowMouseCursor true)
  (bind _returnvalue (UserInterface|CreateWidget "/Game/Menu/UW_YouWin.UW_YouWin_C"))
  (UserInterface|Viewport|AddtoViewport _returnvalue 0)
  (Class|Actor|SetTickablewhenPaused false)
  (Game|SetGamePaused true))

(event Custom|InableAllInput
  ;[1 1 1] Передача управления
  (Input|EnableInput (Pawn|GetControlledPawn) self))

(event Custom|OnServer
  (params (Pawn :type Actor%20Object%20Reference) (Mov :type Float%20%28double-precision%29) (Scale :type Transform))
  ;[1 1 1] Передача движения клиента на сервер
  (bind _asplayer_1 (Utilities|Casting|CastToPlayer1 Pawn))
  (Transformation|AddActorWorldOffset _asplayer_1 (Math|Vector|MakeVector 0.0 Mov 0.0) true)
  (Transformation|SetActorScale3D _asplayer_1 (.scale Scale)))

(event Custom|ReadyForServer
  (params (Ready :type Boolean))
  ;[1 1 1] Вызов из Player controller
  (Variables|Default|SetPlayerReady Ready))

(event EventBeginPlay
  ;[1 1 1] Выставляю камеру
  (Utilities|FlowControl|Delay 1.0)
  (bind _outactors (Actor|GetAllActorsOfClass "/Script/Engine.CameraActor"))
  (Game|Player|SetViewTargetwithBlend (Utilities|Array|Get(acopy) _outactors) 0.0 "VTBlend_Linear" 0.0 false))

(event Input|AxisEvents|InputAxisMoveRight/Left
  (params (AxisValue :type Float%20%28single-precision%29))
  (bind _returnvalue (Pawn|GetControlledPawn))
  (bind _returnvalue_2 (* AxisValue 2e+01))
  ;[1 1 1] Ввод и движение игроков
  (Networking|SwitchHasAuthority
    (:Authority
      (bind _asplayer_1 (Utilities|Casting|CastToPlayer1 _returnvalue))
      (Transformation|AddActorWorldOffset _asplayer_1 (Math|Vector|MakeVector 0.0 _returnvalue_2 0.0) true))
    (:Remote
      (bind _asplayer_1_2 (Utilities|Casting|CastToPlayer1 _returnvalue))
      (Transformation|AddActorWorldOffset _asplayer_1_2 (Math|Vector|MakeVector 0.0 _returnvalue_2 0.0) true)
      (CallFunction|OnServer _asplayer_1_2 _returnvalue_2 (Math|Transform|MakeTransform "0, 0, 0" "0, 0, 0" (Transformation|GetActorScale3D _asplayer_1_2))))))

(event Input|KeyboardEvents|LeftCtrl
  (params (Key :type Key%20Structure :default "None"))
  (:Pressed
    (Development|PrintString "Hello")))

(fn ConstructionScript)