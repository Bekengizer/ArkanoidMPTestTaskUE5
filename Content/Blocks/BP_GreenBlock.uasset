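; BP_GreenBlock is a bonus block that enlarges the player when hit by a BP_Ball.
; On Hit, it applies a velocity-change radial impulse to the hitting component at the impact point.
; It then stretches the Player1 pawn along the Y axis with an absolute actor scale and destroys itself.
; Both outcomes of the Player1 cast continue into this same sequence.
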(event EventBeginPlay
  (|CallParentFunction) ; This node is disabled and will not be called.\nDrag off pins to build functionality.
)

(event Collision|EventActorBeginOverlap
  (params (OtherActor :type Actor%20Object%20Reference))
  (|CallParentFunction OtherActor) ; This node is disabled and will not be called.\nDrag off pins to build functionality.
)

(event EventTick
  (params (DeltaSeconds :type Float%20%28single-precision%29))
  (|CallParentFunction DeltaSeconds) ; This node is disabled and will not be called.\nDrag off pins to build functionality.
)

(event Collision|EventHit
  (params (MyComp :type Primitive%20Component%20Object%20Reference) (Other :type Actor%20Object%20Reference) (OtherComp :type Primitive%20Component%20Object%20Reference) (bSelfMoved :type Boolean) (HitLocation :type Vector :default "0, 0, 0") (HitNormal :type Vector :default "0, 0, 0") (NormalImpulse :type Vector :default "0, 0, 0") (Hit :type Hit%20Result%20Structure%20%28by%20ref%29))
  ;[1 1 1] Бонус Увеличивает размер Игрока
  (Utilities|Casting|CastToBP_Ball Other)
  (bind _asplayer_1 (Utilities|Casting|CastToPlayer1 (Game|Player|GetPlayerPawn 0))
    (:then
      _)
    (:CastFailed
      _))
  (Physics|AddRadialImpulse OtherComp HitLocation 5e+02 1e+03 "RIF_Constant" true)
  (Transformation|SetActorScale3D _asplayer_1 "1.000000,5.000000,1.000000")
  (Actor|DestroyActor))

(fn ConstructionScript
  (|CallParentFunction))