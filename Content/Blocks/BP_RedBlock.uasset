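; BP_RedBlock is a bonus block that increases the ball count when a BP_Ball hits it.
; On hit, it applies a radial impulse at the impact point to the colliding component, then spawns another ball at the original's transform, owned by BP_GameMode.
; The new ball gets replication and movement replication enabled plus an impulse along world X, and the block destroys itself.
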(event EventBeginPlay
  (|CallParentFunction) ; This node is disabled and will not be called.\nDrag off pins to build functionality.
)

(event Collision|EventActorBeginOverlap
  (params (OtherActor :type Actor%20Object%20Reference))
  (|CallParentFunction OtherActor) ; This node is disabled and will not be called.\nDrag off pins to build functionality.
)

(event EventTick
  (params (DeltaSeconds :type Float%20%28single-precision%29))
  (|CallParentFunction DeltaSeconds) ; This node is disabled and will not be called.\nDrag off pins to build functionality.
)

(event Collision|EventHit
  (params (MyComp :type Primitive%20Component%20Object%20Reference) (Other :type Actor%20Object%20Reference) (OtherComp :type Primitive%20Component%20Object%20Reference) (bSelfMoved :type Boolean) (HitLocation :type Vector :default "0, 0, 0") (HitNormal :type Vector :default "0, 0, 0") (NormalImpulse :type Vector :default "0, 0, 0") (Hit :type Hit%20Result%20Structure%20%28by%20ref%29))
  ;[1 1 1] Бонус Увеличивает кол-во шариков
  (bind _asbp_ball (Utilities|Casting|CastToBP_Ball Other))
  (Physics|AddRadialImpulse OtherComp HitLocation 5e+02 1e+03 "RIF_Constant" true)
  (bind _asbp_game_mode (Utilities|Casting|CastToBP_GameMode (Game|GetGameMode)))
  (bind _returnvalue (Game|SpawnActorfromClass "/Game/Ball/BP_Ball.BP_Ball_C" (Transformation|GetActorTransform _asbp_ball) "AdjustIfPossibleButAlwaysSpawn" _asbp_game_mode 0))
  (Networking|SetReplicates _returnvalue true)
  (Class|Actor|SetReplicateMovement _returnvalue true)
  (Physics|AddImpulse (Variables|/Game/Ball/BP_Ball.BP_Ball_C|GetSphere _returnvalue) "500.000000,0.000000,0.000000" "None" true)
  (Actor|DestroyActor))

(fn ConstructionScript
  (|CallParentFunction))